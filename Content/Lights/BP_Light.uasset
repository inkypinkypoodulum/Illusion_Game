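; Light actor that measures how brightly it illuminates the player, for a visibility mechanic.
; Sphere overlaps add or remove it from the player's Lights array and track the player reference.
; Each Tick, a line trace checks occlusion and sets Brightness using a smooth distance falloff over the point light's attenuation radius, or zero when blocked or absent.
; Tick also keeps the sphere radius matched to that attenuation radius.
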(event OnComponentBeginOverlap(Sphere)
  (params (OverlappedComponent :type Primitive%20Component%20Object%20Reference) (OtherActor :type Actor%20Object%20Reference) (OtherComp :type Primitive%20Component%20Object%20Reference) (OtherBodyIndex :type Integer) (bFromSweep :type Boolean) (SweepResult :type Hit%20Result%20Structure%20%28by%20ref%29))
  ;[0 1 0.01373] Adds And Removes the Lights Array From the player character
  (bind _asplayer_character (Utilities|Casting|CastToPlayer_Character OtherActor))
  (Utilities|Array|AddUnique (Variables|/Game/Player/Blueprints/Player_Character.Player_Character_C|GetLights _asplayer_character) self)
  (Variables|Default|SetPlayer _asplayer_character))

(event OnComponentEndOverlap(Sphere)
  (params (OverlappedComponent :type Primitive%20Component%20Object%20Reference) (OtherActor :type Actor%20Object%20Reference) (OtherComp :type Primitive%20Component%20Object%20Reference) (OtherBodyIndex :type Integer))
  ;[0 1 0.01373] Adds And Removes the Lights Array From the player character
  (bind _asplayer_character (Utilities|Casting|CastToPlayer_Character OtherActor))
  (Utilities|Array|RemoveItem (Variables|/Game/Player/Blueprints/Player_Character.Player_Character_C|GetLights _asplayer_character) self)
  (Variables|Default|SetPlayer 0))

(event EventTick
  (params (DeltaSeconds :type Float%20%28single-precision%29))
  (bind _player (Variables|Default|GetPlayer))
  (bind _player_2 (Variables|Default|GetPlayer))
  (bind _pointlight (Variables|Default|GetPointLight))
  (bind _returnvalue (Transformation|GetActorLocation _player))
  (bind _attenuationradius (Variables|/Script/Engine.PointLightComponent|GetAttenuationRadius _pointlight))
  ;[0 1 0.06968] Math Function That dynamically sets the players Visibility Based on location reletive to Lightsource
  (Utilities|FlowControl|Sequence
    (:then_0
      (Utilities|IsValid _player
        (:Is%20Valid
          (bind _outhit (Collision|LineTraceByChannel (Transformation|GetActorLocation) (Math|Vector|MakeVector (.x _returnvalue) (.y _returnvalue) (+ (.z _returnvalue) 3e+01)) "TraceTypeQuery1" false 0 "None"))
          (if (== (.hitactor _outhit) _player_2)
            (Variables|Default|SetBrightness (|(pow((1-(pow((distance/radius),4))),2)) (Math|Float|Min(Float) (Transformation|GetDistanceTo _player_2) _attenuationradius) _attenuationradius))
            (else
              (Variables|Default|SetBrightness 0.0))))
        (:Is%20Not%20Valid
          (Variables|Default|SetBrightness 0.0))))
    (:then_1
      (Components|Sphere|SetSphereRadius (Variables|Default|GetSphere) (Variables|/Script/Engine.PointLightComponent|GetAttenuationRadius (Variables|Default|GetPointLight)) true))))

(fn ConstructionScript)
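; AI controller that runs the AI_BT behavior tree and feeds it how well the AI perceives the player.
; After a short startup delay it writes player pawn 0 to the Blackboard.
; Each tick it reads the player character's visibility and noise level.
; It scales them by the sight and hearing stimulus strengths from AIPerception, writing perceived visibility and noise floats to the Blackboard, or zero when not sensed.
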(event OnPerceptionUpdated(AIPerception)
  (params (UpdatedActors :type Array%20of%20Actor%20Object%20References)))

(event EventBeginPlay
  (AI|RunBehaviorTree "/Game/AI/AI_BT.AI_BT")
  (Utilities|FlowControl|Delay 4.0)
  (CallFunction|SetPlayer (Game|Player|GetPlayerPawn 0)))

(event EventTick
  (params (DeltaSeconds :type Float%20%28single-precision%29))
  (bind _player (Variables|Default|GetPlayer))
  ;[1 1 1] set tick rate low, only updating keys
  (Utilities|FlowControl|Sequence
    (:then_0
      (CallFunction|UpdatePlayerInfo _player))
    (:then_1
      (CallFunction|IsPlayerVisible _player))
    (:then_2
      (CallFunction|IsPlayerHeard _player))))

(fn ConstructionScript)

(fn SetPlayer
  (params (Actor :type Actor%20Object%20Reference))
  (if (!= Actor (Variables|Default|GetPlayer))
    (bind _output_get (Variables|Default|SetPlayer Actor))
    (AI|Components|Blackboard|SetValueasObject (AI|GetBlackboard 0) (Variables|Default|GetPlayerKey) _output_get)))

(fn GetActorsPerception
  (params (AI%20Perception :type AI%20Perception%20Component%20Object%20Reference) (Actor :type Actor%20Object%20Reference) (SenseIndex :type Integer))
  (bind _info (Class|AIPerceptionComponent|GetActorsPerception AI%20Perception Actor))
  (return (AI|GetBlackboard self) (.LastSensedStimuli (Utilities|Struct|BreakActorPerceptionBlueprintInfo _info)) (.Age (Utilities|Struct|BreakAIStimulus (Utilities|Array|Get(acopy) (.LastSensedStimuli (Utilities|Struct|BreakActorPerceptionBlueprintInfo _info)) SenseIndex))) (.ExpirationAge (Utilities|Struct|BreakAIStimulus (Utilities|Array|Get(acopy) (.LastSensedStimuli (Utilities|Struct|BreakActorPerceptionBlueprintInfo _info)) SenseIndex))) (.Strength (Utilities|Struct|BreakAIStimulus (Utilities|Array|Get(acopy) (.LastSensedStimuli (Utilities|Struct|BreakActorPerceptionBlueprintInfo _info)) SenseIndex))) (.StimulusLocation (Utilities|Struct|BreakAIStimulus (Utilities|Array|Get(acopy) (.LastSensedStimuli (Utilities|Struct|BreakActorPerceptionBlueprintInfo _info)) SenseIndex))) (.ReceiverLocation (Utilities|Struct|BreakAIStimulus (Utilities|Array|Get(acopy) (.LastSensedStimuli (Utilities|Struct|BreakActorPerceptionBlueprintInfo _info)) SenseIndex))) (.Tag (Utilities|Struct|BreakAIStimulus (Utilities|Array|Get(acopy) (.LastSensedStimuli (Utilities|Struct|BreakActorPerceptionBlueprintInfo _info)) SenseIndex))) (.bSuccessfullySensed (Utilities|Struct|BreakAIStimulus (Utilities|Array|Get(acopy) (.LastSensedStimuli (Utilities|Struct|BreakActorPerceptionBlueprintInfo _info)) SenseIndex)))))

(fn IsPlayerVisible
  (params (Player :type Actor%20Object%20Reference))
  (Utilities|Casting|CastToPlayer_Character Player)
  (bind (_blackboard _lastsensedstimuli _age _expiration_age _strength _stimulus_location _receiver_location _tag _successfully_sensed) (CallFunction|GetActorsPerception (Variables|Default|GetAIPerception) (Variables|Default|GetPlayer)))
  (AI|Components|Blackboard|SetValueasFloat (AI|GetBlackboard 0) (Utilities|Name|MakeLiteralName "PercievedPlayerVisibility") (Math|Float|SelectFloat (* _strength (Variables|PlayerInfo|GetPlayerInfoVisibility)) 0.0 _successfully_sensed))
  (return))

(fn UpdatePlayerInfo
  (params (Player :type Actor%20Object%20Reference))
  (bind _asplayer_character (Utilities|Casting|CastToPlayer_Character Player))
  (Utilities|FlowControl|Sequence
    (:then_0
      (Variables|PlayerInfo|SetPlayerInfoVisibility (Variables|/Game/Player/Blueprints/Player_Character.Player_Character_C|GetVisibility _asplayer_character)))
    (:then_1
      (Variables|PlayerInfo|SetPlayerInfoCurrentNoiseLevel (Variables|/Game/Player/Blueprints/Player_Character.Player_Character_C|GetCurrent%20Noise%20Level _asplayer_character)))))

(fn IsPlayerHeard
  (params (Player :type Actor%20Object%20Reference))
  (Utilities|Casting|CastToPlayer_Character Player)
  (bind (_blackboard _lastsensedstimuli _age _expiration_age _strength _stimulus_location _receiver_location _tag _successfully_sensed) (CallFunction|GetActorsPerception (Variables|Default|GetAIPerception) (Variables|Default|GetPlayer) 1))
  (AI|Components|Blackboard|SetValueasFloat (AI|GetBlackboard 0) (Utilities|Name|MakeLiteralName "PercievedPlayerNoise") (Math|Float|SelectFloat (* _strength (Variables|PlayerInfo|GetPlayerInfoCurrentNoiseLevel)) 0.0 _successfully_sensed))
  (return))
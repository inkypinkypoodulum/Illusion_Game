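; AI character Blueprint that tracks its own movement speed as a normalized value.
; Each tick it stores its current velocity and speed, then maps that speed to a clamped 0–1 VelocityAlpha.
; The upper bound switches between crouched and standard max walk speed from CharacterMovement, so the alpha stays relative to the current stance.
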(event EventTick
  (params (DeltaSeconds :type Float%20%28single-precision%29))
  (bind _charactermovement (Variables|Character|GetCharacterMovement))
  (bind _output_get (Variables|Default|SetCurrentVelocity (Transformation|GetVelocity)))
  (bind _output_get_2 (Variables|Default|SetCurrentSpeed (Math|Vector|VectorLength _output_get)))
  (Variables|Default|SetVelocityAlpha (Math|Float|Clamp(Float) (Math|Float|NormalizetoRange _output_get_2 0.0 (Math|Float|SelectFloat (Variables|/Script/Engine.CharacterMovementComponent|GetMaxWalkSpeedCrouched _charactermovement) (Variables|/Script/Engine.CharacterMovementComponent|GetMaxWalkSpeed _charactermovement) (Variables|Default|GetbIsCrouched))) 0.0 1.0)))

(fn ConstructionScript)